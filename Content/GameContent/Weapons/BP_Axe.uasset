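; BP_Axe is an axe weapon actor with its own health, which is destroyed when that health runs out.
; Health starts at its maximum on BeginPlay, and the Damage event subtracts the incoming amount.
; Tick polls health every frame to destroy the actor at zero or below, rather than checking inside the Damage event.
; Getter functions expose its HitBox and Mesh.
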(event EventBeginPlay
  (Variables|Default|SetCurrentHealth (Variables|Default|GetMaxHealth)))

(event EventTick
  (params (DeltaSeconds :type Float%20%28single-precision%29))
  (Utilities|FlowControl|Sequence
    (:then_0
      (if (<= (Variables|Default|GetCurrentHealth) 0.0)
        (Actor|DestroyActor)))))

(event EventDamage
  (params (Amount :type Float%20%28double-precision%29))
  (Variables|Default|SetCurrentHealth (- (Variables|Default|GetCurrentHealth) Amount)))

(event Collision|EventActorBeginOverlap
  (params (OtherActor :type Actor%20Object%20Reference)))

(fn ConstructionScript)

(fn GetHitBox
  (return (Variables|Default|GetHitBox)))

(fn GetMesh
  (return (Variables|Default|GetMesh)))